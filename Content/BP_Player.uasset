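; Player character for a melee game where targets are struck on the left or right at three heights.
; Each input turns the mesh and probes close, middle and far collisions to pick a montage, whose notify hits the target and adds score.
; Tick checks both sides for targets, panning and zooming the spring-arm camera with matching focal distance.
; It also handles the Ibuki intro, damage reactions, God Mode and knockdown game over through GameManager.
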(event OnComponentHit(CapsuleComponent)
  (params (HitComponent :type Primitive%20Component%20Object%20Reference) (OtherActor :type Actor%20Object%20Reference) (OtherComp :type Primitive%20Component%20Object%20Reference) (NormalImpulse :type Vector :default "0, 0, 0") (Hit :type Hit%20Result%20Structure%20%28by%20ref%29))
  ;[1 1 1] (削除するかもしれない)ターゲットが体に当たった時の処理
)

(event Custom|InitializeInput
  (bind _returnvalue (Game|GetPlayerController 0))
  (bind _returnvalue_2 (PlayerController|LocalPlayerSubsystems|GetEnhancedInputLocalPlayerSubsystem _returnvalue))
  ;[1 1 1] Enhanced Input の初期化
  (Utilities|FlowControl|Sequence
    (:then_0
      (Input|EnableInput _returnvalue))
    (:then_1
      (Utilities|IsValid _returnvalue_2
        (:Is%20Valid
          (Input|AddMappingContext _returnvalue_2 "/Game/IMC_Default.IMC_Default" 0 "(bIgnoreAllPressedKeysUntilRelease=True,bForceImmediately=False,bNotifyUserSettings=False)"))))))

(event Custom|Move%20Camera
  (params (TargetOffsetY :type Vector) (TargetArmLength :type Float%20%28double-precision%29))
  (bind _springarm (Variables|Default|GetSpringArm))
  (bind _springarm_2 (Variables|Default|GetSpringArm))
  ;[1 1 1] カメラを左右に動かす
  (Timeline|Timeline PlayFromStart
    (:Update
      (Variables|/Script/Engine.SpringArmComponent|SetTargetOffset _springarm (Math|Vector|Lerp(Vector) (Variables|/Script/Engine.SpringArmComponent|GetTargetOffset _springarm_2) TargetOffsetY 0.02))
      (Variables|/Script/Engine.SpringArmComponent|SetTargetArmLength _springarm (Math|Float|Lerp (Variables|/Script/Engine.SpringArmComponent|GetTargetArmLength _springarm_2) TargetArmLength 0.02)))))

(event Custom|Unfreeze
  ;[1 1 1] 入力を無効/有効にする
  (Variables|Default|SetCanControl true))

(event Custom|Ibuki
  ;[1 1 1] 息吹
  (CallFunction|SwitchPlayerDirection "NewEnumerator2")
  (Animation|Montage|PlayMontage (Variables|Character|GetMesh) "/Game/Characters/Rosales/Animations/AM_Ibuki.AM_Ibuki"
    (:OnCompleted
      (Class|GameManagerCpp|ChangeStatus (Variables|Default|GetGameManager) "InGame"))))

(event Custom|Damage
  (params (Damage :type Integer))
  ;[1 1 1] ダメージ処理（God Mode の時はライフが0以下でも死なない）
  (bind _output_get (Variables|Default|SetLife (- (Variables|Default|GetLife) Damage)))
  (CallFunction|Hit)
  (Development|PrintString (Utilities|String|BuildString(Integer) "Damaged. " "Current Life: " _output_get))
  (if (not (Variables|Default|GetGodMode))
    (Default|CallOnChangeLife (Variables|Default|GetLife) (Variables|Default|GetMaxLife)) ; UI を更新する
    (if (<= (Variables|Default|GetLife) 0)
      (CallFunction|GameOver))))

(event Custom|GameOver
  ;[1 1 1] ゲームオーバー処理
  (CallFunction|Freeze)
  (Class|GameManagerCpp|ChangeStatus (Variables|Default|GetGameManager) "GameOver")
  (Collision|SetCollisionEnabled (Variables|Collision|GetCapsuleComponent) "NoCollision")
  (bind _montage (CallFunction|RandomPickMontage (Variables|Default|GetKnockDown%20Mongage%20List)))
  (Animation|Montage|PlayMontage (Variables|Character|GetMesh) _montage))

(event Custom|Attack
  (bind _target (Variables|Default|GetTarget))
  ;[1 1 1] 攻撃のアニメーションを再生して、ターゲットを攻撃する
  (Animation|Montage|PlayMontage (Variables|Character|GetMesh) (Variables|Default|GetAttackMontage)
    (:OnNotifyBegin
      (Utilities|IsValid _target
        (:Is%20Valid
          (Class|ATargetBase|Attacked _target)
          (Class|GameManagerCpp|AddScore (Variables|Default|GetGameManager) (Variables|/Script/petitcon21.ATargetBase|GetScore _target)) ; 得点を更新する
        )))))

(event Custom|ProcessInput
  (params (Far%20Collision :type Box%20Component%20Object%20Reference) (Middle%20Collision :type Box%20Component%20Object%20Reference) (Close%20Collision :type Box%20Component%20Object%20Reference) (Far%20Attack%20Montage :type Anim%20Montage%20Object%20Reference) (Middle%20Attack%20Montage :type Anim%20Montage%20Object%20Reference) (Close%20Attack%20Montage :type Anim%20Montage%20Object%20Reference))
  ;[1 1 1] 攻撃の入力を処理する
  (bind _target (CallFunction|GetTarget Close%20Collision))
  (bind _output_get (Variables|Default|SetTarget _target))
  (Utilities|IsValid _output_get
    (:Is%20Valid
      (Variables|Default|SetAttackMontage Close%20Attack%20Montage)
      (CallFunction|Attack))
    (:Is%20Not%20Valid
      (bind _target_2 (CallFunction|GetTarget Middle%20Collision))
      (bind _output_get_2 (Variables|Default|SetTarget _target_2))
      (Utilities|IsValid _output_get_2
        (:Is%20Valid
          (Variables|Default|SetAttackMontage Middle%20Attack%20Montage)
          (CallFunction|Attack))
        (:Is%20Not%20Valid
          (bind _target_3 (CallFunction|GetTarget Far%20Collision))
          (bind _output_get_3 (Variables|Default|SetTarget _target_3))
          (Utilities|IsValid _output_get_3
            (:Is%20Valid
              (Variables|Default|SetAttackMontage Far%20Attack%20Montage)
              (CallFunction|Attack))
            (:Is%20Not%20Valid
              (CallFunction|Attack))))))))

(event Custom|Hit
  ;[1 1 1] くらった時の処理
  (bind _montage (CallFunction|RandomPickMontage (Variables|Default|GetDamage%20Montage%20List)))
  (Animation|Montage|PlayMontage (Variables|Character|GetMesh) _montage))

(event Custom|SwitchPlayerDirection
  (params (PlayerDirection :type E_PlayerDirection%20Enum :default "NewEnumerator0"))
  ;[1 1 1] プレイヤーの向きを変える（ここではターゲット角度を設定するのみで、実際の回転は Tick で行う）
  (if (Utilities|Enum|NotEqual(Enum) PlayerDirection (Variables|Default|GetPlayerDirection))
    (bind _output_get (Variables|Default|SetPlayerDirection PlayerDirection))
    (switch Utilities|FlowControl|Switch|SwitchonE_PlayerDirection _output_get
      (:NewEnumerator0
        (Variables|Default|SetTargetRotation (Variables|Default|GetPlayerDirectionRight)))
      (:NewEnumerator1
        (Variables|Default|SetTargetRotation (Variables|Default|GetPlayerDirectionLeft)))
      (:NewEnumerator2
        (Variables|Default|SetTargetRotation (Variables|Default|GetInitialMeshRotation))))))

(event Custom|CheckTargets
  ;[1 1 1] 左右にターゲットがあるかチェックする
  (Variables|Default|SetIsTargetOnRightSide (> (Utilities|Array|Length (Collision|GetOverlappingActors (Variables|Default|GetRight) "/Script/petitcon21.ATargetBase" :!class /Script/Engine.PrimitiveComponent)) 0))
  (Variables|Default|SetIsTargetOnLeftSide (> (Utilities|Array|Length (Collision|GetOverlappingActors (Variables|Default|GetLeft) "/Script/petitcon21.ATargetBase" :!class /Script/Engine.PrimitiveComponent)) 0)))

(event Custom|SetCameraPan
  ;[1 1 1] カメラの位置を決める（実際には動かさない）
  (Variables|Default|SetLastCameraPan (Variables|Default|GetCameraPan))
  (if (and (Variables|Default|GetIsTargetOnLeftSide) (Variables|Default|GetIsTargetOnRightSide))
    (Variables|Default|SetCameraPan "NewEnumerator2")
    (elif (Variables|Default|GetIsTargetOnRightSide)
      (Variables|Default|SetCameraPan "NewEnumerator0")
      (elif (Variables|Default|GetIsTargetOnLeftSide)
        (Variables|Default|SetCameraPan "NewEnumerator1")
        (else
          (Variables|Default|SetCameraPan "NewEnumerator3"))))))

(event Custom|MoveCameraBasedOnPan
  ;[1 1 1] CameraPan の状態によってカメラを動かす
  (if (Utilities|Enum|NotEqual(Enum) (Variables|Default|GetCameraPan) (Variables|Default|GetLastCameraPan))
    (switch Utilities|FlowControl|Switch|SwitchonE_CameraPan (Variables|Default|GetCameraPan)
      (:NewEnumerator0
        (CallFunction|MoveCamera "0.000000,-150.000000,0.000000" 2.2e+02))
      (:NewEnumerator1
        (CallFunction|MoveCamera "0.000000,150.000000,0.000000" 2.2e+02))
      (:NewEnumerator2
        (CallFunction|MoveCamera "0, 0, 0" 3.5e+02))
      (:NewEnumerator3
        (CallFunction|MoveCamera "0, 0, 0" 2.2e+02)))
    (CallFunction|AdjustFocalDistance)))

(event Custom|Freeze
  ;[1 1 1] 入力を無効/有効にする
  (Variables|Default|SetCanControl false))

(event Input|EnhancedActionEvents|EnhancedInputActionIA_RightHigh
  (params (ActionValue :type Boolean) (ElapsedSeconds :type Float%20%28double-precision%29) (TriggeredSeconds :type Float%20%28double-precision%29) (InputAction :type Input%20Action%20Object%20Reference :default "/Game/IA_RightHigh.IA_RightHigh"))
  ;[1 1 1] 入力→攻撃
  (if (Variables|Default|GetCanControl)
    (CallFunction|SwitchPlayerDirection "NewEnumerator0")
    (CallFunction|ProcessInput (Variables|Default|GetRightUpFarCollision) (Variables|Default|GetRightUpMiddleCollision) (Variables|Default|GetRightUpCloseCollision) "/Game/Characters/Rosales/Animations/AM_RoundhouseKick_High.AM_RoundhouseKick_High" "/Game/Characters/Rosales/Animations/AM_Jab_High.AM_Jab_High" "/Game/Characters/Rosales/Animations/AM_Cross_High.AM_Cross_High")))

(event Input|EnhancedActionEvents|EnhancedInputActionIA_RightMiddle
  (params (ActionValue :type Boolean) (ElapsedSeconds :type Float%20%28double-precision%29) (TriggeredSeconds :type Float%20%28double-precision%29) (InputAction :type Input%20Action%20Object%20Reference :default "/Game/IA_RightMiddle.IA_RightMiddle"))
  ;[1 1 1] 入力→攻撃
  (if (Variables|Default|GetCanControl)
    (CallFunction|SwitchPlayerDirection "NewEnumerator0")
    (CallFunction|ProcessInput (Variables|Default|GetRightMiddleFarCollision) (Variables|Default|GetRightMiddleMiddleCollision) (Variables|Default|GetRightMiddleCloseCollision) "/Game/Characters/Rosales/Animations/AM_SideKick_Middle.AM_SideKick_Middle" "/Game/Characters/Rosales/Animations/AM_Cross_Middle.AM_Cross_Middle" "/Game/Characters/Rosales/Animations/AM_Jab_Middle.AM_Jab_Middle")))

(event Input|EnhancedActionEvents|EnhancedInputActionIA_RightLow
  (params (ActionValue :type Boolean) (ElapsedSeconds :type Float%20%28double-precision%29) (TriggeredSeconds :type Float%20%28double-precision%29) (InputAction :type Input%20Action%20Object%20Reference :default "/Game/IA_RightLow.IA_RightLow"))
  ;[1 1 1] 入力→攻撃
  (if (Variables|Default|GetCanControl)
    (CallFunction|SwitchPlayerDirection "NewEnumerator0")
    (CallFunction|ProcessInput (Variables|Default|GetRightLowFarCollision) (Variables|Default|GetRightLowMiddleCollision) (Variables|Default|GetRightLowCloseCollision) "/Game/Characters/Rosales/Animations/AM_RoundhouseKick_Low.AM_RoundhouseKick_Low" "/Game/Characters/Rosales/Animations/AM_RoundhouseKick_Low.AM_RoundhouseKick_Low" "/Game/Characters/Rosales/Animations/AM_RoundhouseKick_Low.AM_RoundhouseKick_Low")))

(event Input|EnhancedActionEvents|EnhancedInputActionIA_LeftHigh
  (params (ActionValue :type Boolean) (ElapsedSeconds :type Float%20%28double-precision%29) (TriggeredSeconds :type Float%20%28double-precision%29) (InputAction :type Input%20Action%20Object%20Reference :default "/Game/IA_LeftHigh.IA_LeftHigh"))
  ;[1 1 1] 入力→攻撃
  (if (Variables|Default|GetCanControl)
    (CallFunction|SwitchPlayerDirection "NewEnumerator1")
    (CallFunction|ProcessInput (Variables|Default|GetLeftUpFarCollision) (Variables|Default|GetLeftUpMiddleCollision) (Variables|Default|GetLeftUpCloseCollision) "/Game/Characters/Rosales/Animations/AM_RoundhouseKick_High.AM_RoundhouseKick_High" "/Game/Characters/Rosales/Animations/AM_Jab_High.AM_Jab_High" "/Game/Characters/Rosales/Animations/AM_Cross_High.AM_Cross_High")))

(event Input|EnhancedActionEvents|EnhancedInputActionIA_LeftMiddle
  (params (ActionValue :type Boolean) (ElapsedSeconds :type Float%20%28double-precision%29) (TriggeredSeconds :type Float%20%28double-precision%29) (InputAction :type Input%20Action%20Object%20Reference :default "/Game/IA_LeftMiddle.IA_LeftMiddle"))
  ;[1 1 1] 入力→攻撃
  (if (Variables|Default|GetCanControl)
    (CallFunction|SwitchPlayerDirection "NewEnumerator1")
    (CallFunction|ProcessInput (Variables|Default|GetLeftMiddleFarCollision) (Variables|Default|GetLeftMiddleMiddleCollision) (Variables|Default|GetLeftMiddleCloseCollision) "/Game/Characters/Rosales/Animations/AM_SideKick_Middle.AM_SideKick_Middle" "/Game/Characters/Rosales/Animations/AM_Jab_Middle.AM_Jab_Middle" "/Game/Characters/Rosales/Animations/AM_Cross_Middle.AM_Cross_Middle")))

(event Input|EnhancedActionEvents|EnhancedInputActionIA_LeftLow
  (params (ActionValue :type Boolean) (ElapsedSeconds :type Float%20%28double-precision%29) (TriggeredSeconds :type Float%20%28double-precision%29) (InputAction :type Input%20Action%20Object%20Reference :default "/Game/IA_LeftLow.IA_LeftLow"))
  ;[1 1 1] 入力→攻撃
  (if (Variables|Default|GetCanControl)
    (CallFunction|SwitchPlayerDirection "NewEnumerator1")
    (CallFunction|ProcessInput (Variables|Default|GetLeftLowFarCollision) (Variables|Default|GetLeftLowMiddleCollision) (Variables|Default|GetLeftLowCloseCollision) "/Game/Characters/Rosales/Animations/AM_RoundhouseKick_Low.AM_RoundhouseKick_Low" "/Game/Characters/Rosales/Animations/AM_RoundhouseKick_Low.AM_RoundhouseKick_Low" "/Game/Characters/Rosales/Animations/AM_RoundhouseKick_Low.AM_RoundhouseKick_Low")))

(event EventBeginPlay
  (CallFunction|InitializeInput)
  (CallFunction|SetCameraPan)
  (CallFunction|AdjustFocalDistance))

(event EventTick
  (params (DeltaSeconds :type Float%20%28single-precision%29))
  (CallFunction|CheckTargets) ; ターゲットの位置を調べる
  (CallFunction|SetCameraPan) ; カメラの位置を決める
  (CallFunction|MoveCameraBasedonPan) ; カメラを動かす
  (Transformation|SetRelativeRotation (Variables|Character|GetMesh) (Math|Interpolation|RInterpTo (Variables|/Script/Engine.SceneComponent|GetRelativeRotation (Variables|Character|GetMesh)) (Variables|Default|GetTargetRotation) DeltaSeconds (Variables|Default|GetRotateInterpSpeed)) false false) ; プレイヤーを回転させる
)

(fn ConstructionScript
  (Utilities|FlowControl|Sequence
    (:then_0
      ;[1 1 1] 変数の初期化
      (bind _output_get (Variables|Default|SetInitialMeshRotation (Variables|/Script/Engine.SceneComponent|GetRelativeRotation (Variables|Character|GetMesh))))
      (Variables|Default|SetTargetRotation _output_get))
    (:then_1
      (Variables|Default|SetLife (Variables|Default|GetMaxLife)))
    (:then_2
      ;[1 1 1] 息吹→ゲーム開始のイベントバインド
      (bind _returnvalue (Actor|GetActorOfClass "/Game/BP_GameManager.BP_GameManager_C"))
      (bind _output_get_2 (Variables|Default|SetGameManager _returnvalue))
      (EventDispatchers|BindEventtoOnIntroduction _output_get_2 (EventDispatchers|CreateEvent :!event Custom|Ibuki))
      (EventDispatchers|BindEventtoOnGameStart _output_get_2 (EventDispatchers|CreateEvent :!event Custom|Unfreeze)))
    (:then_3
      (EventDispatchers|BindEventtoOnChangeLife (EventDispatchers|CreateEvent (Variables|Default|GetGameManager) :!event ChangeLife)))))

(fn GetTarget
  (params (Collision :type Box%20Component%20Object%20Reference))
  (for _array_element (Collision|GetOverlappingActors Collision "/Script/petitcon21.ATargetBase" :!class /Script/Engine.PrimitiveComponent)
    (bind _asatarget_base (Utilities|Casting|CastToATargetBase _array_element)
      (:then
        (return _asatarget_base))
      (:CastFailed
        (return 0))))
  (return 0))

(fn RandomPickMontage
  (params (MontageList :type Array%20of%20Anim%20Montage%20Object%20References))
  (return (.OutItem (Utilities|Array|Random MontageList))))

(fn AdjustFocalDistance
  (Utilities|Struct|SetmembersinPostProcessSettings (Variables|/Script/Engine.CameraComponent|GetPostProcessSettings (Variables|Default|GetCamera)) (Variables|/Script/Engine.SpringArmComponent|GetTargetArmLength (Variables|Default|GetSpringArm))))