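; BP_Jar is a breakable jar that damages the player on impact and can be shattered by attacks.
; Any hit stops physics, damages a BP_Player if struck, then swaps the jar for BP_Jar_Crash.
; Attacked does the same swap with a stronger Explode value, both after a tiny bug-workaround delay.
; A dynamic material turns the outline red while overlapping a component tagged AttackTargetCollision, and black afterwards.
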(event OnComponentHit(StaticMesh)
  (params (HitComponent :type Primitive%20Component%20Object%20Reference) (OtherActor :type Actor%20Object%20Reference) (OtherComp :type Primitive%20Component%20Object%20Reference) (NormalImpulse :type Vector :default "0, 0, 0") (Hit :type Hit%20Result%20Structure%20%28by%20ref%29))
  ;[1 1 1] プレイヤーに当たった時はダメージを与えて割れる。それ以外に当たった時は割れる。
  (Physics|SetSimulatePhysics HitComponent false)
  (bind _asbp_player (Utilities|Casting|CastToBP_Player OtherActor)
    (:then
      (Default|Damage _asbp_player (Variables|Default|GetDamage)))
    (:CastFailed
      _))
  (Utilities|FlowControl|Delay 0.0005) ; バグ回避のために少し遅らせる
  (bind _returnvalue (Game|SpawnActorfromClass "/Game/BP_Jar_Crash.BP_Jar_Crash_C" (Transformation|GetWorldTransform (Variables|Default|GetStaticMesh)) "Undefined" "MultiplyWithRoot" 0 0))
  (Default|Explode _returnvalue 0.0)
  (Actor|DestroyActor))

(event OnComponentBeginOverlap(StaticMesh)
  (params (OverlappedComponent :type Primitive%20Component%20Object%20Reference) (OtherActor :type Actor%20Object%20Reference) (OtherComp :type Primitive%20Component%20Object%20Reference) (OtherBodyIndex :type Integer) (bFromSweep :type Boolean) (SweepResult :type Hit%20Result%20Structure%20%28by%20ref%29))
  (CallFunction|ChangeOutlineColor OtherComp "(R=1.000000,G=0.031896,B=0.031896,A=1.000000)"))

(event OnComponentEndOverlap(StaticMesh)
  (params (OverlappedComponent :type Primitive%20Component%20Object%20Reference) (OtherActor :type Actor%20Object%20Reference) (OtherComp :type Primitive%20Component%20Object%20Reference) (OtherBodyIndex :type Integer))
  (CallFunction|ChangeOutlineColor OtherComp "(R=0.000000,G=0.000000,B=0.000000,A=1.000000)"))

(event Custom|SaveMI
  ;[1 1 1] アウトライン用のMIを保持する
  (bind _returnvalue (Rendering|Material|CreateDynamicMaterialInstance (Variables|Default|GetOutline) 0 0 "None" :!class /Script/Engine.PrimitiveComponent))
  (Variables|Default|SetMIDMesh _returnvalue))

(event Custom|ChangeOutlineColor
  (params (OtherComponent :type Primitive%20Component%20Object%20Reference) (Color :type Linear%20Color%20Structure))
  ;[1 1 1] アウトライン用MIの色を変える
  (if (Components|ComponentHasTag OtherComponent "AttackTargetCollision")
    (Rendering|Material|SetVectorParameterValue (Variables|Default|GetMIDMesh) "Outline Color" Color :!class /Script/Engine.MaterialInstanceDynamic)))

(event EventAttacked
  ;[1 1 1] 攻撃された場合は爆発する
  (Utilities|FlowControl|Delay 0.0005) ; バグ回避のために少し遅らせる
  (bind _returnvalue (Game|SpawnActorfromClass "/Game/BP_Jar_Crash.BP_Jar_Crash_C" (Transformation|GetWorldTransform (Variables|Default|GetStaticMesh)) "Undefined" "MultiplyWithRoot" 0 0))
  (Default|Explode _returnvalue 1.5e+02)
  (Actor|DestroyActor))

(event EventBeginPlay
  (CallFunction|SaveMI))

(fn ConstructionScript)