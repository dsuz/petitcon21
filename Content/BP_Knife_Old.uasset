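; BP_Knife_Old is a knife projectile actor that damages the player on impact.
; On BeginPlay its physics capsule is launched along the actor's forward vector at Speed.
; A capsule hit on a BP_Player calls that player's Hit and destroys the knife, while other hits are ignored.
; Its own Hit event also destroys it through Die.
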(event OnComponentHit(Capsule)
  (params (HitComponent :type Primitive%20Component%20Object%20Reference) (OtherActor :type Actor%20Object%20Reference) (OtherComp :type Primitive%20Component%20Object%20Reference) (NormalImpulse :type Vector :default "0, 0, 0") (Hit :type Hit%20Result%20Structure%20%28by%20ref%29))
  (bind _asbp_player (Utilities|Casting|CastToBP_Player OtherActor))
  (Default|Hit _asbp_player)
  (CallFunction|Die))

(event Custom|Hit
  (CallFunction|Die))

(event Custom|Die
  (Actor|DestroyActor))

(event EventBeginPlay
  (Physics|SetPhysicsLinearVelocity (Variables|Default|GetCapsule) (* (Transformation|GetActorForwardVector) (Variables|Default|GetSpeed)) false "None"))

(event Collision|EventActorBeginOverlap
  (params (OtherActor :type Actor%20Object%20Reference)))

(event EventTick
  (params (DeltaSeconds :type Float%20%28single-precision%29)))

(fn ConstructionScript)