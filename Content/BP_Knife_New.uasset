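; BP_Knife_New is a knife actor that damages BP_Player when it hits them, then destroys itself.
; Hitting anything else also destroys it, unless the Attacked event has flagged it as struck by the player.
; When attacked, it switches to gravity and physics-only collision, flies spinning along its mesh's right vector via set linear and angular velocities, and is destroyed by a short timer.
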(event OnComponentHit(StaticMesh)
  (params (HitComponent :type Primitive%20Component%20Object%20Reference) (OtherActor :type Actor%20Object%20Reference) (OtherComp :type Primitive%20Component%20Object%20Reference) (NormalImpulse :type Vector :default "0, 0, 0") (Hit :type Hit%20Result%20Structure%20%28by%20ref%29))
  ;[1 1 1] プレイヤーに当たった時はダメージを与えて消え、それ以外に当たった時はそのまま消える
  (bind _asbp_player (Utilities|Casting|CastToBP_Player OtherActor)
    (:then
      (Default|Damage _asbp_player (Variables|Default|GetDamage))
      (Actor|DestroyActor :!label _label))
    (:CastFailed
      (if (not (Variables|Default|GetHitByPlayer)) ; プレイヤーに攻撃される前にどこかに当たった場合は消す
        (goto _label)))))

(event Custom|CustomEvent
  ;[1 1 1] 攻撃された時の処理
  (Actor|DestroyActor))

(event Custom|FlyAway
  (bind _staticmesh (Variables|Default|GetStaticMesh))
  ;[1 1 1] 周りながら飛んでいく
  (Utilities|FlowControl|Sequence
    (:then_0
      (Physics|SetEnableGravity (Variables|Default|GetStaticMesh) true)
      (Collision|SetCollisionEnabled (Variables|Default|GetStaticMesh) "PhysicsOnly"))
    (:then_1
      (Physics|SetPhysicsLinearVelocity _staticmesh (* (Math|Vector|GetRightVector _staticmesh) 6e+02) false "None"))
    (:then_2
      (Class|PrimitiveComponent|SetPhysicsAngularVelocityinDegrees (Variables|Default|GetStaticMesh) "600.000000,600.000000,600.000000" false "None"))))

(event EventAttacked
  ;[1 1 1] 攻撃された時の処理
  (Variables|Default|SetHitByPlayer true)
  (CallFunction|FlyAway)
  (Utilities|Time|SetTimerbyEvent (delegate Custom|CustomEvent) 1.0))

(fn ConstructionScript)