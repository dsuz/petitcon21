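; BP_Knife is a hazard that damages BP_Player on hit and destroys itself, or vanishes on hitting anything else unless the player struck it first.
; Attacked marks it as hit, plays a sound, sends it spinning sideways under physics and gravity, and shortens its lifespan.
; Dynamic outline materials cached at BeginPlay turn red while overlapping a component tagged AttackTargetCollision, and black afterwards.
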(event OnComponentHit(StaticMesh)
  (params (HitComponent :type Primitive%20Component%20Object%20Reference) (OtherActor :type Actor%20Object%20Reference) (OtherComp :type Primitive%20Component%20Object%20Reference) (NormalImpulse :type Vector :default "0, 0, 0") (Hit :type Hit%20Result%20Structure%20%28by%20ref%29))
  ;[1 1 1] プレイヤーに当たった時はダメージを与えて消え、それ以外に当たった時はそのまま消える
  (bind _asbp_player (Utilities|Casting|CastToBP_Player OtherActor)
    (:then
      (Default|Damage _asbp_player (Variables|Default|GetDamage))
      (Actor|DestroyActor :!label _label))
    (:CastFailed
      (if (not (Variables|Default|GetHitByPlayer)) ; プレイヤーに攻撃される前にどこかに当たった場合は消す
        (goto _label)))))

(event OnComponentBeginOverlap(StaticMesh)
  (params (OverlappedComponent :type Primitive%20Component%20Object%20Reference) (OtherActor :type Actor%20Object%20Reference) (OtherComp :type Primitive%20Component%20Object%20Reference) (OtherBodyIndex :type Integer) (bFromSweep :type Boolean) (SweepResult :type Hit%20Result%20Structure%20%28by%20ref%29))
  (CallFunction|ChangeOutlineColor OtherComp "(R=1.000000,G=0.000000,B=0.000000,A=1.000000)"))

(event OnComponentEndOverlap(StaticMesh)
  (params (OverlappedComponent :type Primitive%20Component%20Object%20Reference) (OtherActor :type Actor%20Object%20Reference) (OtherComp :type Primitive%20Component%20Object%20Reference) (OtherBodyIndex :type Integer))
  (CallFunction|ChangeOutlineColor OtherComp))

(event Custom|FlyAway
  (bind _staticmesh (Variables|Default|GetStaticMesh))
  (bind _staticmesh_2 (Variables|Default|GetStaticMesh))
  ;[1 1 1] 周りながら飛んでいく
  (Utilities|FlowControl|Sequence
    (:then_0
      (Physics|SetEnableGravity (Variables|Default|GetStaticMesh) true)
      (Collision|SetCollisionEnabled _staticmesh_2 "PhysicsOnly")
      (Class|PrimitiveComponent|SetConstraintMode _staticmesh_2 "None"))
    (:then_1
      (Physics|SetPhysicsLinearVelocity _staticmesh (* (Math|Vector|GetRightVector _staticmesh) 6e+02) false "None"))
    (:then_2
      (Class|PrimitiveComponent|SetPhysicsAngularVelocityinDegrees (Variables|Default|GetStaticMesh) "600.000000,600.000000,600.000000" false "None"))))

(event Custom|ChangeOutlineColor
  (params (OtherComponent :type Primitive%20Component%20Object%20Reference) (Color :type Linear%20Color%20Structure))
  ;[1 1 1] アウトライン用MIの色を変える
  (if (Components|ComponentHasTag OtherComponent "AttackTargetCollision")
    (for _array_element (Variables|Default|GetMIDMeshArray)
      (Rendering|Material|SetVectorParameterValue _array_element "Outline Color" Color :!class /Script/Engine.MaterialInstanceDynamic))))

(event Custom|PlayHitAudio
  ;[1 1 1] 効果音を鳴らす
  (Audio|PlaySoundatLocation (Variables|Default|GetHitAudioCue) (Transformation|GetWorldLocation (Variables|Default|GetStaticMesh)) "0, 0, 0" 1.0 1.0 0.0 0 0 0 0))

(event Custom|SaveMI
  (bind _outline (Variables|Default|GetOutline))
  ;[1 1 1] アウトライン用のMIを保持する
  (bind _result (Math|Integer|DecrementInt (Rendering|Material|GetNumMaterials _outline))
    (:%20%20
      (for _index (range 0 _result)
        (bind _returnvalue (Rendering|Material|CreateDynamicMaterialInstance _outline _index 0 "None" :!class /Script/Engine.PrimitiveComponent))
        (Utilities|Array|Add (Variables|Default|GetMIDMeshArray) _returnvalue)))))

(event EventAttacked
  ;[1 1 1] 攻撃された時の処理
  (Variables|Default|SetHitByPlayer true)
  (CallFunction|PlayHitAudio)
  (CallFunction|FlyAway)
  (Class|ATargetBase|ResetLifeSpan 1.0))

(event EventBeginPlay
  (CallFunction|SaveMI))

(fn ConstructionScript)