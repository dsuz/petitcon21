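; Game manager that runs the stage flow from intro through play to clear or game over, and advances to the next stage or Title.
; BeginPlay caches the player and stage manager, binds game-state and score events, and creates the main UI.
; A looping timer confirms stage clear once no targets remain and the player is alive.
; Intro and clear play Level Sequences with the player bound by tag, alongside UI fades.
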(event Custom|Start
  (Class|StageManagerBase|Start (Variables|Default|GetStageManager) (Variables|Default|GetStageNumber)))

(event Custom|StopSpawiningTarget
  ;[1 1 1] ターゲットの生成を止める処理
  (Class|StageManagerBase|Pause (Variables|Default|GetStageManager)))

(event Custom|ValidateStageClear
  ;[1 1 1] ステージクリアしているかチェックする。クリアしたら入力を無効にして演出を再生する。
  (bind _returnvalue (Utilities|Time|SetTimerbyEvent (delegate Custom|CheckStageClear) 1.0 true))
  (Variables|Default|SetValidateStageClearHandle _returnvalue))

(event Custom|CheckStageClear
  ;[1 1 1] ステージクリアしているかチェックする。クリアしたら入力を無効にして演出を再生する。
  (bind _outactors (Actor|GetAllActorsOfClass "/Script/petitcon21.ATargetBase"))
  (if (> (Utilities|Array|Length _outactors) 0)
    (Development|PrintString "Stage Finished. Checking stage clear condition...")
    (else
      (if (> (Variables|/Game/BP_Player.BP_Player_C|GetLife (Variables|Default|GetPlayer)) 0)
        (Development|PrintString "Clear.")
        (Class|GameManagerCpp|ChangeStatus "Clear")
        (Default|Freeze (Variables|Default|GetPlayer))
        (CallFunction|StageClear)
        (else
          (Development|PrintString "Player is dead.")))
      (Utilities|Time|ClearandInvalidateTimerbyHandle (Variables|Default|GetValidateStageClearHandle)))))

(event Custom|GameOver
  ;[1 1 1] ゲームオーバー時の処理
  (CallFunction|StopSpawiningTarget)
  (bind _returnvalue (UserInterface|CreateWidget "/Game/WBP_GameOver.WBP_GameOver_C"))
  (UserInterface|Viewport|AddtoViewport _returnvalue 0))

(event Custom|GoToNextStage
  ;[1 1 1] 次のステージに行く処理。現在が最終ステージならタイトルに戻る。
  (if (> (Variables|/Script/petitcon21.StageManagerBase|GetLastStageNumber (Variables|Default|GetStageManager)) (Variables|Default|GetStageNumber))
    (Math|Integer|IncrementInt (Variables|Default|GetStageNumber)
      (:%20%20
        (Class|GameManagerCpp|ChangeStatus "Intro")))
    (else
      (Game|OpenLevel(byName) "Title"))))

(event Custom|Introduction
  (bind _levelsequenceactor (Variables|Default|GetLevelSequenceActor))
  (bind _mainui (Variables|Default|GetMainUI))
  ;[1 1 1] プレイ開始演出を再生する
  (UserInterface|Animation|PlayAnimation _mainui (Variables|/Game/WBP_MainUI.WBP_MainUI_C|GetFadeIn _mainui) 0.0 1 "Forward" 1.0 false)
  (Class|LevelSequenceActor|SetSequence (Variables|Default|GetLevelSequenceActor) (Variables|Default|GetOpeningSequence))
  (Class|LevelSequenceActor|AddBindingbyTag _levelsequenceactor "Player" (Variables|Default|GetPlayer) false)
  (Sequencer|Player|Play (Variables|/Script/LevelSequence.LevelSequenceActor|GetSequencePlayer _levelsequenceactor) :!class /Script/MovieScene.MovieSceneSequencePlayer))

(event Custom|ChangeScore
  (bind _returnvalue (Class|GameManagerCpp|GetScore))
  (Default|ChangeScore (Variables|Default|GetMainUI) _returnvalue))

(event Custom|ChangeLife
  (params (CurrentLife :type Integer) (MaxLife :type Integer))
  ;[1 1 1] ライフのUIを更新する
  (Default|ChangeLife (Variables|Default|GetMainUI) CurrentLife MaxLife))

(event Custom|StageClear
  (bind _mainui (Variables|Default|GetMainUI))
  (bind _levelsequenceactor (Variables|Default|GetLevelSequenceActor))
  (bind _fadein (Variables|/Game/WBP_MainUI.WBP_MainUI_C|GetFadeIn _mainui))
  ;[1 1 1] ステージクリア演出を再生する
  (bind _returnvalue (Animation|GetPlayLength _fadein))
  (UserInterface|Animation|PlayAnimation _mainui _fadein _returnvalue 1 "Reverse" 1.0 false) ; UIを隠す
  (Class|LevelSequenceActor|SetSequence (Variables|Default|GetLevelSequenceActor) (Variables|Default|GetStageClearSequence)) ; シーケンサーを再生する
  (Class|LevelSequenceActor|AddBindingbyTag _levelsequenceactor "Player" (Variables|Default|GetPlayer) false)
  (Sequencer|Player|Play (Variables|/Script/LevelSequence.LevelSequenceActor|GetSequencePlayer _levelsequenceactor) :!class /Script/MovieScene.MovieSceneSequencePlayer))

(event EventBeginPlay
  (bind _returnvalue (Actor|GetActorOfClass "/Game/BP_Player.BP_Player_C"))
  (Variables|Default|SetPlayer _returnvalue)
  (bind _returnvalue_2 (Actor|GetActorOfClass "/Game/BP_StageManager.BP_StageManager_C"))
  (bind _output_get (Variables|Default|SetStageManager _returnvalue_2))
  (EventDispatchers|BindEventtoOnTargetGenerationComplete _output_get (EventDispatchers|CreateEvent :!event Custom|ValidateStageClear))
  (EventDispatchers|BindEventtoOnGameStart (delegate Custom|Start))
  (EventDispatchers|BindEventtoOnGameOver (EventDispatchers|CreateEvent :!event Custom|GameOver))
  (EventDispatchers|BindEventtoOnIntroduction (EventDispatchers|CreateEvent :!event Custom|Introduction))
  (bind _returnvalue_3 (UserInterface|CreateWidget "/Game/WBP_MainUI.WBP_MainUI_C"))
  (bind _output_get_2 (Variables|Default|SetMainUI _returnvalue_3))
  (UserInterface|Viewport|AddtoViewport _output_get_2 0)
  (EventDispatchers|BindEventtoOnChangeScore (delegate Custom|ChangeScore)))

(fn ConstructionScript
  (bind _returnvalue (Actor|GetActorOfClass "/Script/LevelSequence.LevelSequenceActor"))
  (Variables|Default|SetLevelSequenceActor _returnvalue))