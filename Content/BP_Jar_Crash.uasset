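; BP_Jar_Crash is the shattered form of a jar that bursts with a given power and removes itself 1.5 seconds after spawning.
; Explode plays one of two crash sounds, chosen by whether Power is positive.
; It then spawns an FS_MasterField at the ExplosionLocation component's transform, sets its radial magnitude to Power and triggers it, using a field system to drive the break-up.
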(event Custom|CustomEvent
  ;[1 1 1] 一定時間後に消えるようにする
  (Actor|DestroyActor))

(event Custom|Explode
  (params (Power :type Float%20%28double-precision%29))
  ;[1 1 1] 爆発させる
  (CallFunction|PlayHitAudio Power)
  (bind _returnvalue (Game|SpawnActorfromClass "/Engine/EditorResources/FieldNodes/FS_MasterField.FS_MasterField_C" (Transformation|GetWorldTransform (Variables|Default|GetExplosionLocation)) "Undefined" "MultiplyWithRoot" 0 0))
  (Variables|/Engine/EditorResources/FieldNodes/FS_MasterField.FS_MasterField_C|SetRadial%20Magnitude _returnvalue Power)
  (Variables|/Engine/EditorResources/FieldNodes/FS_MasterField.FS_MasterField_C|SetActivationType _returnvalue "NewEnumerator4")
  (Default|CETrigger _returnvalue))

(event Custom|PlayHitAudio
  (params (Power :type Float%20%28double-precision%29))
  (bind _returnvalue (Transformation|GetActorLocation))
  ;[1 1 1] 割れたSEを鳴らす
  (if (> Power 0.0)
    (Audio|PlaySoundatLocation (Variables|Default|GetCrashSound2) _returnvalue "0, 0, 0" 1.0 1.0 0.0 0 0 0 0)
    (else
      (Audio|PlaySoundatLocation (Variables|Default|GetCrashSound1) _returnvalue "0, 0, 0" 1.0 1.0 0.0 0 0 0 0))))

(event EventBeginPlay
  ;[1 1 1] 一定時間後に消えるようにする
  (Utilities|Time|SetTimerbyEvent (delegate Custom|CustomEvent) 1.5))

(fn ConstructionScript)